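; BP_PedeSegment is an actor for a pede segment that tries to attach segments when a character touches it.
; Its capsule's begin-overlap event casts the other actor to BaseCharacter and calls AttemptAttachSegments with it.
; The result is printed on screen as debug output.
; The actor overlap event only forwards to the parent, and the construction script adds nothing of its own.
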(event `self.ReceiveActorBeginOverlap`
  (params (OtherActor :type "Actor Object Reference"))
  (`parent.ReceiveActorBeginOverlap` OtherActor))

(event `self.CapsuleComponent.OnComponentBeginOverlap`
  (params (OverlappedComponent :type "PrimitiveComponent Object Reference") (OtherActor :type "Actor Object Reference") (OtherComp :type "PrimitiveComponent Object Reference") (OtherBodyIndex :type Integer) (bFromSweep :type Boolean) (SweepResult :type "HitResult Structure (by ref)"))
  (bind _asbase_character (cast `BaseCharacter` OtherActor))
  (bind _returnvalue (`self.AttemptAttachSegments` _asbase_character))
  (`KismetSystemLibrary.PrintString` (`KismetStringLibrary.Conv_BoolToString` _returnvalue) true true (struct :`G` 0.66 :`B` 1.0 :`A` 1.0) 15.0))

(fn `UserConstructionScript`
  (`parent.UserConstructionScript`))