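; Base character Blueprint with a custom movement component and an Ability System Component, providing a simple sprint toggle.
; StartSprint and EndSprint raise and restore the movement component's max fly speed, leaving walk speed untouched.
; Tick prints the current max speed every frame as debug output.
; A GAS chain that would apply GE_PlusLevel to itself is left unconnected and never runs.
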(event `StartSprint`
  (`CustomCharacterMovementComponent.SetMaxFlySpeed` (`self.GetCustomCharacterMovementComponent`) 1200.0))

(event `EndSprint`
  (`CustomCharacterMovementComponent.SetMaxFlySpeed` (`self.GetCustomCharacterMovementComponent`) 600.0))

(event `self.ReceiveTick`
  (params (DeltaSeconds :type "Float (single-precision)"))
  (`KismetSystemLibrary.PrintString` (`KismetStringLibrary.Conv_DoubleToString` (`MovementComponent.GetMaxSpeed` (`self.GetCustomCharacterMovementComponent`)))))

(fn `UserConstructionScript`)