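; Player controller for the main game that turns the pawn toward the mouse cursor or gamepad stick and moves it along its facing.
; It adds an Enhanced Input mapping context and switches between gamepad and keyboard based on the last key pressed.
; Tick sets control rotation from the look stick or deprojected cursor position, flattened to yaw.
; Move inputs drive the pawn's forward vector, with stick magnitude remapped past a deadzone.
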(event `self.ReceiveBeginPlay`
  ;[1 1 1] Add Mapping Context
  (`EnhancedInputSubsystemInterface.AddMappingContext` (subsystem `EnhancedInputLocalPlayerSubsystem`) "/Game/Input/IMC_MainGame.IMC_MainGame" 0 (struct)))

(event `Key|AnyKey`
  (params (Key :type "Key Structure"))
  ;[1 1 1] Switch between gamepad and keyboard
  (:`Pressed`
    (set `self.bUsingGamepad` (`KismetInputLibrary.Key_IsGamepadKey` Key))))

(event `self.ReceiveTick`
  (params (DeltaSeconds :type "Float (single-precision)"))
  (bind (_worldlocation _worlddirection _returnvalue) (`self.DeprojectMousePositionToWorld`))
  (bind _returnvalue_2 (`|GetInputActionValue`))
  (bind (_x _y) (`KismetMathLibrary.BreakVector2D` _returnvalue_2))
  ;[1 1 1] Tick: Turn in direction (cursor/gamepad stick)
  (if (`self.bUsingGamepad`)
    (if (> (`KismetMathLibrary.VSize2D` _returnvalue_2) (`self.MinStickInputToLook`))
      (`self.SetControlRotation` (`KismetMathLibrary.MakeRotFromX` (`KismetMathLibrary.MakeVector` _y _x))))
    (elif _returnvalue
      (`self.SetControlRotation` (`KismetMathLibrary.MakeRotFromX` (`KismetMathLibrary.MakeVector` (.x (- _worldlocation (`self.K2_GetActorLocation` (`self.K2_GetPawn`)))) (.y (- _worldlocation (`self.K2_GetActorLocation` (`self.K2_GetPawn`))))))))))

(event `EnhancedInput|/Game/Input/IA_KeyMove`
  (params (ActionValue :type "Float (double-precision)") (ElapsedSeconds :type "Float (double-precision)") (TriggeredSeconds :type "Float (double-precision)") (InputAction :type "InputAction Object Reference" :default "/Game/Input/IA_KeyMove.IA_KeyMove"))
  (bind _returnvalue (`self.K2_GetPawn`))
  ;[1 1 1] Move Forward
  ;;[1 1 1] Keyboard
  (:`Triggered`
    (`Pawn.AddMovementInput` _returnvalue (`self.GetActorForwardVector` _returnvalue) ActionValue false)))

(event `EnhancedInput|/Game/Input/IA_StickMove`
  (params (ActionValue :type "Vector2D Structure") (ElapsedSeconds :type "Float (double-precision)") (TriggeredSeconds :type "Float (double-precision)") (InputAction :type "InputAction Object Reference" :default "/Game/Input/IA_StickMove.IA_StickMove"))
  (bind _returnvalue (`KismetMathLibrary.VSize2D` ActionValue))
  (bind _returnvalue_2 (`self.K2_GetPawn`))
  (bind _minstickinputtomove (`self.MinStickInputToMove`))
  ;[1 1 1] Move Forward
  ;;[1 1 1] Controller
  (:`Triggered`
    (if (> _returnvalue _minstickinputtomove)
      (`Pawn.AddMovementInput` _returnvalue_2 (`self.GetActorForwardVector` _returnvalue_2) (`KismetMathLibrary.MapRangeClamped` _returnvalue _minstickinputtomove 1.0 0.0 1.0) false))))

(fn `UserConstructionScript`)