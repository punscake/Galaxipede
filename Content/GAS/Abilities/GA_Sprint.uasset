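; GA_Sprint is a gameplay ability that lets a BP_BaseCharacter sprint while the input is held.
; On activation it commits, applies GE_Sprint and sets the custom movement component's max fly speed to the product of two attribute values.
; It ends on input release or when a watched attribute falls below a threshold.
; If committed, ending resets fly speed from an attribute and removes effects granting Combat.Sprinting.
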(event `self.K2_ActivateAbility`
  (bind _avataractor (`self.AvatarActor`))
  (bind _returnvalue (`AbilitySystemBlueprintLibrary.GetAbilitySystemComponent` _avataractor))
  (set `self.bAbilityCommited` false)
  (bind _asbp_base_character (cast `/Game/Actors/BP_BaseCharacter` (`self.GetAvatarActorFromActorInfo`))
    (:`then`
      (set `self.AvatarActor` _asbp_base_character)
      (`self.K2_CommitAbility`)
      (set `self.bAbilityCommited` true)
      (`self.BP_ApplyGameplayEffectToOwner` "/Game/GAS/Effects/GE_Sprint.GE_Sprint_C")
      (`CustomCharacterMovementComponent.SetMaxFlySpeed` (`BaseCharacter.GetCustomCharacterMovementComponent` _avataractor) (* (`.ReturnValue` (`AbilitySystemComponent.GetGameplayAttributeValue` _returnvalue (struct :`AttributeName` "MaxSpeed" :`Attribute` "/Script/Galaxipede.MovementAttributeSet:MaxSpeed" :`AttributeOwner` "/Script/CoreUObject.Class'\"/Script/Galaxipede.MovementAttributeSet\"'"))) (`.ReturnValue` (`AbilitySystemComponent.GetGameplayAttributeValue` _returnvalue (struct :`AttributeName` "SurgeSpeedMulti" :`Attribute` "/Script/Galaxipede.MovementAttributeSet:SurgeSpeedMulti" :`AttributeOwner` "/Script/CoreUObject.Class'\"/Script/Galaxipede.MovementAttributeSet\"'")))))
      (`AbilityTask_WaitInputRelease.WaitInputRelease` false
        (:`then`
          (bind (_asynctaskproxy _bmatchescomparison) (`AbilityTask_WaitAttributeChangeThreshold.WaitForAttributeChangeThreshold` (struct :`AttributeName` "SurgeTime" :`Attribute` "/Script/Galaxipede.MovementAttributeSet:SurgeTime" :`AttributeOwner` "/Script/CoreUObject.Class'\"/Script/Galaxipede.MovementAttributeSet\"'") "LessThan" 0.0 true null)
            (:`OnChange`
              (if _bmatchescomparison
                (`self.K2_EndAbility`)))))
        (:`OnRelease`
          (`self.K2_EndAbility`))))
    (:`CastFailed`
      (`self.K2_EndAbility`))))

(event `self.K2_OnEndAbility`
  (params (bWasCancelled :type Boolean))
  (bind _avataractor (`self.AvatarActor`))
  (if (`self.bAbilityCommited`)
    (`CustomCharacterMovementComponent.SetMaxFlySpeed` (`BaseCharacter.GetCustomCharacterMovementComponent` _avataractor) (`.ReturnValue` (`AbilitySystemComponent.GetGameplayAttributeValue` (`AbilitySystemBlueprintLibrary.GetAbilitySystemComponent` _avataractor) (struct :`AttributeName` "MaxSpeed" :`Attribute` "/Script/Galaxipede.MovementAttributeSet:MaxSpeed" :`AttributeOwner` "/Script/CoreUObject.Class'\"/Script/Galaxipede.MovementAttributeSet\"'"))))
    (`self.BP_RemoveGameplayEffectFromOwnerWithGrantedTags` (struct :`GameplayTags` (struct :`(TagName` "Combat.Sprinting"))))))